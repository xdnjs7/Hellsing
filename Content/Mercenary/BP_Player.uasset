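; Player Blueprint for a 2D flipbook character that walks along world X and Y and swings an axe.
; Movement axes drive movement input and switch between Idle and Walk based on IsMoving, which WASD key events update; A and D also flip the sprite's facing.
; Left click starts the Axe flipbook and blocks movement, while Tick watches for its last frame to return to Idle.
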(event EventBeginPlay
  (Utilities|Casting|CastToHellsing_PC (Game|GetPlayerController 0)))

(event Collision|EventActorBeginOverlap
  (params (OtherActor :type Actor%20Object%20Reference)))

(event EventTick
  (params (DeltaSeconds :type Float%20%28single-precision%29))
  (if (and (Variables|Default|GetIsAttack) (>= (+ (Class|PaperFlipbookComponent|GetPlaybackPositioninFrames (Variables|Default|GetSprite)) 1) (Class|PaperFlipbook|GetNumFrames (Class|PaperFlipbookComponent|GetFlipbook (Variables|Default|GetSprite)))))
    (Variables|Default|SetIsAttack false)
    (Sprite|SetFlipbook (Variables|Default|GetSprite) "/Game/Resources/PaperFlipBook/Idle.Idle")))

(event Input|ActionEvents|InputActionLeftClick
  (params (Key :type Key%20Structure :default "None"))
  (:Pressed
    (Variables|Default|SetIsAttack true)
    (if (Variables|Default|GetIsAttack)
      (Sprite|SetFlipbook (Variables|Default|GetSprite) "/Game/Resources/PaperFlipBook/Axe.Axe")
      (Components|Timeline|SetPlayRate (Variables|Default|GetSprite) 1.0))))

(event Input|ActionEvents|InputActionRightClick
  (params (Key :type Key%20Structure :default "None")))

(event Input|AxisEvents|InputAxisMoveForward
  (params (AxisValue :type Float%20%28single-precision%29))
  (if (not (Variables|Default|GetIsAttack))
    (Pawn|Input|AddMovementInput "0.000000,1.000000,0.000000" AxisValue false)
    (if (Variables|Default|GetIsMoving)
      (Sprite|SetFlipbook (Variables|Default|GetSprite) "/Game/Resources/PaperFlipBook/Walk.Walk")
      (else
        (Sprite|SetFlipbook (Variables|Default|GetSprite) "/Game/Resources/PaperFlipBook/Idle.Idle")))))

(event Input|AxisEvents|InputAxisMoveRight
  (params (AxisValue :type Float%20%28single-precision%29))
  (if (not (Variables|Default|GetIsAttack))
    (Pawn|Input|AddMovementInput "1.000000,0.000000,0.000000" AxisValue false)
    (if (Variables|Default|GetIsMoving)
      (Sprite|SetFlipbook (Variables|Default|GetSprite) "/Game/Resources/PaperFlipBook/Walk.Walk")
      (else
        (Sprite|SetFlipbook (Variables|Default|GetSprite) "/Game/Resources/PaperFlipBook/Idle.Idle")))))

(event Input|KeyboardEvents|A
  (params (Key :type Key%20Structure :default "None"))
  ;[1 1 1 1 50] 이동버튼 입력 감지
  (:Pressed
    (Variables|Default|SetIsMoving (Math|Boolean|ORBoolean (Variables|Default|GetIsWPressed) (Variables|Default|GetIsAPressed) (Variables|Default|GetIsSPressed) (Variables|Default|GetIsDPressed)))
    (Transformation|SetWorldRotation (Variables|Default|GetSprite) "0.000000,180.000000,0.000000" false false))
  (:Released
    (Variables|Default|SetIsMoving (Math|Boolean|ANDBoolean (Variables|Default|GetIsWPressed) (Variables|Default|GetIsAPressed) (Variables|Default|GetIsSPressed) (Variables|Default|GetIsDPressed)))))

(event Input|KeyboardEvents|D
  (params (Key :type Key%20Structure :default "None"))
  ;[1 1 1 1 50] 이동버튼 입력 감지
  (:Pressed
    (Variables|Default|SetIsMoving (Math|Boolean|ORBoolean (Variables|Default|GetIsWPressed) (Variables|Default|GetIsAPressed) (Variables|Default|GetIsSPressed) (Variables|Default|GetIsDPressed)))
    (Transformation|SetWorldRotation (Variables|Default|GetSprite) "0, 0, 0" false false))
  (:Released
    (Variables|Default|SetIsMoving (Math|Boolean|ANDBoolean (Variables|Default|GetIsWPressed) (Variables|Default|GetIsAPressed) (Variables|Default|GetIsSPressed) (Variables|Default|GetIsDPressed)))))

(event Input|KeyboardEvents|W
  (params (Key :type Key%20Structure :default "None"))
  ;[1 1 1 1 50] 이동버튼 입력 감지
  (:Pressed
    (Variables|Default|SetIsMoving (Math|Boolean|ORBoolean (Variables|Default|GetIsWPressed) (Variables|Default|GetIsAPressed) (Variables|Default|GetIsSPressed) (Variables|Default|GetIsDPressed))))
  (:Released
    (Variables|Default|SetIsMoving (Math|Boolean|ANDBoolean (Variables|Default|GetIsWPressed) (Variables|Default|GetIsAPressed) (Variables|Default|GetIsSPressed) (Variables|Default|GetIsDPressed)))))

(event Input|KeyboardEvents|S
  (params (Key :type Key%20Structure :default "None"))
  ;[1 1 1 1 50] 이동버튼 입력 감지
  (:Pressed
    (Variables|Default|SetIsMoving (Math|Boolean|ORBoolean (Variables|Default|GetIsWPressed) (Variables|Default|GetIsAPressed) (Variables|Default|GetIsSPressed) (Variables|Default|GetIsDPressed))))
  (:Released
    (Variables|Default|SetIsMoving (Math|Boolean|ANDBoolean (Variables|Default|GetIsWPressed) (Variables|Default|GetIsAPressed) (Variables|Default|GetIsSPressed) (Variables|Default|GetIsDPressed)))))

(fn ConstructionScript)