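; BP_Bullet is a short-lived projectile actor with no damage logic of its own.
; Each Tick it applies a fixed local offset along the negated forward vector of the player character's current rotation, without sweep or delta-time scaling.
; Because that direction is re-read every frame and applied in local space, its path depends on both player and bullet rotation.
; It destroys itself after a brief delay or when its StaticMesh registers a hit.
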(event OnComponentHit(StaticMesh)
  (params (HitComponent :type Primitive%20Component%20Object%20Reference) (OtherActor :type Actor%20Object%20Reference) (OtherComp :type Primitive%20Component%20Object%20Reference) (NormalImpulse :type Vector :default "0, 0, 0") (Hit :type Hit%20Result%20Structure%20%28by%20ref%29))
  (Actor|DestroyActor))

(event EventBeginPlay
  (Utilities|FlowControl|Delay 0.5)
  (Actor|DestroyActor self))

(event Collision|EventActorBeginOverlap
  (params (OtherActor :type Actor%20Object%20Reference)))

(event EventTick
  (params (DeltaSeconds :type Float%20%28single-precision%29))
  (Transformation|AddActorLocalOffset self (* -1e+01 (Math|Vector|GetForwardVector (Transformation|GetActorRotation (Game|GetPlayerCharacter 0)))) false false))

(fn ConstructionScript)