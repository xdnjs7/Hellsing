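; Player character for exploration, using a Paper2D sprite that walks, flips with A/D and attacks.
; Movement axes apply input outside attacks and pick Walk or Idle from WASD flags, whose release check chains equality tests rather than ORing them.
; Left click plays Axe for a 0.4-second movement lock, then spawns BP_Bullet offset by facing.
; Sphere and Capsule overlaps hide components until overlap ends; hitting TM1 resets movement and attack state.
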(event OnComponentBeginOverlap(Sphere)
  (params (OverlappedComponent :type Primitive%20Component%20Object%20Reference) (OtherActor :type Actor%20Object%20Reference) (OtherComp :type Primitive%20Component%20Object%20Reference) (OtherBodyIndex :type Integer) (bFromSweep :type Boolean) (SweepResult :type Hit%20Result%20Structure%20%28by%20ref%29))
  (Rendering|SetVisibility OtherComp false true))

(event OnComponentEndOverlap(Sphere)
  (params (OverlappedComponent :type Primitive%20Component%20Object%20Reference) (OtherActor :type Actor%20Object%20Reference) (OtherComp :type Primitive%20Component%20Object%20Reference) (OtherBodyIndex :type Integer))
  (Rendering|SetVisibility OtherComp true true))

(event OnComponentBeginOverlap(Capsule)
  (params (OverlappedComponent :type Primitive%20Component%20Object%20Reference) (OtherActor :type Actor%20Object%20Reference) (OtherComp :type Primitive%20Component%20Object%20Reference) (OtherBodyIndex :type Integer) (bFromSweep :type Boolean) (SweepResult :type Hit%20Result%20Structure%20%28by%20ref%29))
  (Rendering|SetVisibility OtherComp false true))

(event OnComponentEndOverlap(Capsule)
  (params (OverlappedComponent :type Primitive%20Component%20Object%20Reference) (OtherActor :type Actor%20Object%20Reference) (OtherComp :type Primitive%20Component%20Object%20Reference) (OtherBodyIndex :type Integer))
  (Rendering|SetVisibility OtherComp true true))

(event OnComponentHit(CapsuleComponent)
  (params (HitComponent :type Primitive%20Component%20Object%20Reference) (OtherActor :type Actor%20Object%20Reference) (OtherComp :type Primitive%20Component%20Object%20Reference) (NormalImpulse :type Vector :default "0, 0, 0") (Hit :type Hit%20Result%20Structure%20%28by%20ref%29))
  (Utilities|Casting|CastToTM1 OtherActor)
  (Variables|Default|SetPlayerMoving false)
  (Variables|Default|SetIsAttack false)
  (Variables|Default|SetIsWPressed false)
  (Variables|Default|SetIsAPressed false)
  (Variables|Default|SetIsSPressed false)
  (Variables|Default|SetIsDPressed false))

(event Custom|CreateBullet
  (bind _sprite (Variables|Default|GetSprite))
  (bind _returnvalue (Transformation|GetWorldTransform _sprite))
  (if (> (.yaw (.rotation _returnvalue)) 9e+01)
    (Game|SpawnActorfromClass "/Game/Explore/BP_Bullet.BP_Bullet_C" (Math|Transform|MakeTransform (+ (.location _returnvalue) "50.000000,0.000000,-150.000000") (Math|Rotator|MakeRotator (.roll (.rotation _returnvalue)) (.pitch (.rotation _returnvalue)) (.yaw (.rotation _returnvalue))) "1.000000,1.000000,1.000000") "Undefined" "MultiplyWithRoot" 0 0)
    (else
      (Game|SpawnActorfromClass "/Game/Explore/BP_Bullet.BP_Bullet_C" (Math|Transform|MakeTransform (- (.location _returnvalue) "50.000000,0.000000,0.000000") (Math|Rotator|MakeRotator (.roll (.rotation _returnvalue)) (.pitch (.rotation _returnvalue)) (.yaw (.rotation _returnvalue))) "1.000000,1.000000,1.000000") "Undefined" "MultiplyWithRoot" 0 0))))

(event EventBeginPlay
  (Utilities|Casting|CastToHellsing_PC (Game|GetPlayerController 0))
  (Variables|Default|SetPlayerMoving false)
  (Variables|Default|SetIsAttack false)
  (Variables|Default|SetIsWPressed false)
  (Variables|Default|SetIsAPressed false)
  (Variables|Default|SetIsSPressed false)
  (Variables|Default|SetIsDPressed false))

(event EventTick
  (params (DeltaSeconds :type Float%20%28single-precision%29)))

(event Input|ActionEvents|InputActionLeftClick
  (params (Key :type Key%20Structure))
  (:Pressed
    (Variables|Default|SetIsAttack true)
    (Sprite|SetFlipbook (Variables|Default|GetSprite) "/Game/Resources/PaperFlipBook/Axe.Axe")
    (Utilities|FlowControl|Delay 0.4)
    (Sprite|SetFlipbook (Variables|Default|GetSprite) "/Game/Resources/PaperFlipBook/Idle.Idle")
    (Variables|Default|SetIsAttack false)
    (CallFunction|CreateBullet)))

(event Input|AxisEvents|InputAxisMoveForward
  (params (AxisValue :type Float%20%28single-precision%29))
  (if (not (Variables|Default|GetIsAttack))
    (Pawn|Input|AddMovementInput "0.000000,1.000000,0.000000" AxisValue false)
    (if (Variables|Default|GetPlayerMoving)
      (Sprite|SetFlipbook (Variables|Default|GetSprite) "/Game/Resources/PaperFlipBook/Walk.Walk")
      (else
        (Sprite|SetFlipbook (Variables|Default|GetSprite) "/Game/Resources/PaperFlipBook/Idle.Idle")))))

(event Input|AxisEvents|InputAxisMoveRight
  (params (AxisValue :type Float%20%28single-precision%29))
  (if (not (Variables|Default|GetIsAttack))
    (Pawn|Input|AddMovementInput "1.000000,0.000000,0.000000" AxisValue false)
    (if (Variables|Default|GetPlayerMoving)
      (Sprite|SetFlipbook (Variables|Default|GetSprite) "/Game/Resources/PaperFlipBook/Walk.Walk")
      (else
        (Sprite|SetFlipbook (Variables|Default|GetSprite) "/Game/Resources/PaperFlipBook/Idle.Idle")))))

(event Input|KeyboardEvents|A
  (params (Key :type Key%20Structure))
  ;[1 1 1 1 50] 이동버튼 입력 감지
  (:Pressed
    (Variables|Default|SetIsAPressed true)
    (Variables|Default|SetPlayerMoving true)
    (Transformation|SetWorldRotation (Variables|Default|GetSprite) "0.000000,180.000000,0.000000" false false))
  (:Released
    (Variables|Default|SetIsAPressed false)
    (if (== (== (Variables|Default|GetIsWPressed) (Variables|Default|GetIsAPressed)) (== (Variables|Default|GetIsSPressed) (Variables|Default|GetIsDPressed)))
      (Variables|Default|SetPlayerMoving false)
      (Sprite|SetFlipbook (Variables|Default|GetSprite) "/Game/Resources/PaperFlipBook/Idle.Idle")
      (else
        (Variables|Default|SetPlayerMoving true)))))

(event Input|KeyboardEvents|D
  (params (Key :type Key%20Structure))
  ;[1 1 1 1 50] 이동버튼 입력 감지
  (:Pressed
    (Variables|Default|SetIsDPressed true)
    (Variables|Default|SetPlayerMoving true)
    (Transformation|SetWorldRotation (Variables|Default|GetSprite) "0, 0, 0" false false))
  (:Released
    (Variables|Default|SetIsDPressed false)
    (if (== (== (Variables|Default|GetIsWPressed) (Variables|Default|GetIsAPressed)) (== (Variables|Default|GetIsSPressed) (Variables|Default|GetIsDPressed)))
      (Variables|Default|SetPlayerMoving false)
      (Sprite|SetFlipbook (Variables|Default|GetSprite) "/Game/Resources/PaperFlipBook/Idle.Idle")
      (else
        (Variables|Default|SetPlayerMoving true)))))

(event Input|KeyboardEvents|W
  (params (Key :type Key%20Structure))
  ;[1 1 1 1 50] 이동버튼 입력 감지
  (:Pressed
    (Variables|Default|SetIsWPressed true)
    (Variables|Default|SetPlayerMoving true))
  (:Released
    (Variables|Default|SetIsWPressed false)
    (if (== (== (Variables|Default|GetIsWPressed) (Variables|Default|GetIsAPressed)) (== (Variables|Default|GetIsSPressed) (Variables|Default|GetIsDPressed)))
      (Variables|Default|SetPlayerMoving false)
      (Sprite|SetFlipbook (Variables|Default|GetSprite) "/Game/Resources/PaperFlipBook/Idle.Idle")
      (else
        (Variables|Default|SetPlayerMoving true)))))

(event Input|KeyboardEvents|S
  (params (Key :type Key%20Structure))
  ;[1 1 1 1 50] 이동버튼 입력 감지
  (:Pressed
    (Variables|Default|SetIsSPressed true)
    (Variables|Default|SetPlayerMoving true))
  (:Released
    (Variables|Default|SetIsSPressed false)
    (if (== (== (Variables|Default|GetIsWPressed) (Variables|Default|GetIsAPressed)) (== (Variables|Default|GetIsSPressed) (Variables|Default|GetIsDPressed)))
      (Variables|Default|SetPlayerMoving false)
      (Sprite|SetFlipbook (Variables|Default|GetSprite) "/Game/Resources/PaperFlipBook/Idle.Idle")
      (else
        (Variables|Default|SetPlayerMoving true)))))

(fn ConstructionScript)

(fn Attacking)